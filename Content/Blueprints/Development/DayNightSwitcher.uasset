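; Development actor that toggles a level between day and night lighting each time any actor begins overlapping it.
; On BeginPlay it caches the referenced directional light's intensity and color as the daytime look.
; Each overlap flips IsNight, switching between that cached look and a hardcoded dim, pale-cyan night light, then recaptures the referenced skylight so ambient lighting follows the change.
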(event `self.ReceiveBeginPlay`
  (bind _lightcomponent (`Light.LightComponent` (`self.DirectionalLight`)))
  ;[1 1 1] Get Default Light Values (Color / Intensity)
  (set `self.OriginalDirectionalLightIntensity` (`LightComponentBase.Intensity` _lightcomponent))
  (set `self.OriginalDirectionalLightColor` (`LightComponentBase.GetLightColor` _lightcomponent)))

(event `self.ReceiveActorBeginOverlap`
  (params (OtherActor :type "Actor Object Reference"))
  (bind _lightcomponent (`Light.LightComponent` (`self.DirectionalLight`)))
  (bind _lightcomponent_2 (`Light.LightComponent` (`self.DirectionalLight`)))
  (if (`self.IsNight`)
    ;[1 1 1] Set Daylight
    (`LightComponent.SetIntensity` _lightcomponent (`self.OriginalDirectionalLightIntensity`))
    (`LightComponent.SetLightColor` _lightcomponent (`self.OriginalDirectionalLightColor`) true)
    (`SkyLightComponent.RecaptureSky` (`SkyLight.LightComponent` (`self.SkyLight`)))
    (set `self.IsNight` false)
    (else
      ;[1 1 1] Set Nightlight
      (`LightComponent.SetIntensity` _lightcomponent_2 0.005)
      (`LightComponent.SetLightColor` _lightcomponent_2 (struct :`R` 0.515 :`G` 0.932498 :`B` 1.0 :`A` 1.0) true)
      (`SkyLightComponent.RecaptureSky` (`SkyLight.LightComponent` (`self.SkyLight`)))
      (set `self.IsNight` true))))

(fn `UserConstructionScript`)